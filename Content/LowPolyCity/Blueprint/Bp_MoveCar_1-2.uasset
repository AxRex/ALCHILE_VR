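; Car mover actor that drives itself along a spline path in the low-poly city.
; On BeginPlay it finds a Bp_SplinePathLoop_2 actor and starts a timeline with play rate scaled by TimeToComplete.
; Each update maps the timeline track to a distance along the spline and sets the actor's transform there, sampling location in world space but rotation in local space.
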(event `self.ReceiveBeginPlay`
  (bind _returnvalue (`GameplayStatics.GetActorOfClass` "/Game/LowPolyCity/Blueprint/Bp_SplinePathLoop_2.Bp_SplinePathLoop_2_C"))
  (set `self.Spline Ref_2` _returnvalue)
  (`self.Move Object`))

(event `Move Object`
  (bind _spline (`/Game/LowPolyCity/Blueprint/Bp_SplinePathLoop_2.Spline` (`self.Spline Ref_2`)))
  (`TimelineComponent.SetPlayRate` (`self.Move Objetc To Timeline`) (/ 1.0 (`self.Time to complete`)))
  (bind (_direction _move_track) (`Timeline|Move Objetc to Timeline`)
    (:`Update`
      (bind _returnvalue (`KismetMathLibrary.Lerp` 0.0 (`SplineComponent.GetSplineLength` (`/Game/LowPolyCity/Blueprint/Bp_SplinePathLoop_2.Spline` (`self.Spline Ref_2`))) _move_track))
      (`self.K2_SetActorTransform` (`KismetMathLibrary.MakeTransform` (`SplineComponent.GetLocationAtDistanceAlongSpline` _spline _returnvalue "World") (`SplineComponent.GetRotationAtDistanceAlongSpline` _spline _returnvalue "Local"))))))

(fn `UserConstructionScript`)